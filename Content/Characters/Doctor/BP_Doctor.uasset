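; BP_Doctor is a PaperZD character with Enhanced Input movement, dash and attack, plus print-only stubs for parry and fly-through.
; BeginPlay adds the input mapping and HUD, positions the camera and caches the animation instance for Dash and Attack node jumps.
; Horizontal input flips facing and moves the spring arm to follow, replacing per-tick camera updates.
; Dash briefly raises walk speed, with a timeline value gating its cooldown.
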(event `self.ReceiveBeginPlay`
  (bind (_returnvalue_x _returnvalue_y _returnvalue_z) (`KismetMathLibrary.BreakVector` (`self.K2_GetActorLocation`)))
  ;[0 0 0] BeginPlay
  (`|ExecutionSequence`
    (:`then_0`
      (bind _asplayer_controller (cast `PlayerController` (`self.GetController`)))
      (message `EnhancedInputSubsystemInterface.AddMappingContext` (pcsubsystem `EnhancedInputLocalPlayerSubsystem` _asplayer_controller) "/Game/Input/IMC_Main.IMC_Main" 0 (struct)))
    (:`then_1`
      (bind _returnvalue (`|CreateWidget` "/Game/UI/WB_HUD.WB_HUD_C"))
      (`UserWidget.AddToViewport` _returnvalue 0))
    (:`then_2`
      (`SceneComponent.K2_SetWorldLocation` (`self.SpringArm`) (`KismetMathLibrary.MakeVector` 0.0 _returnvalue_y _returnvalue_z) false false))
    (:`then_3`
      (set `self.PaperZD ABP` (`PaperZDAnimationComponent.AnimInstance` (`self.AnimationComponent`))))))

(event `self.ReceiveTick`
  (params (DeltaSeconds :type "Float (single-precision)"))
  ;[1 1 1] disconnected this from tick, now only updates when you move, we can manually update it if the character moves without user input, e.g they get knocked back by something or you dash in a particular direction
)

(event `EnhancedInput|/Game/Input/Actions/IA_Movement`
  (params (ActionValue :type "Vector2D Structure") (ElapsedSeconds :type "Float (double-precision)") (TriggeredSeconds :type "Float (double-precision)") (InputAction :type "InputAction Object Reference" :default "/Game/Input/Actions/IA_Movement.IA_Movement"))
  (bind (_returnvalue_x _returnvalue_y _returnvalue_z) (`KismetMathLibrary.BreakVector` (`self.K2_GetActorLocation`)))
  ;[0 0 0] IMC Main
  (:`Triggered`
    (`self.AddMovementInput` (`KismetMathLibrary.MakeVector` ActionValue_X ActionValue_Y))
    (`/Engine/EditorBlueprintResources/StandardMacros.CompareFloat` ActionValue_Y
      (:`>`
        (`self.K2_SetActorRotation` (struct :`Yaw` 90.0)))
      (:`<`
        (`self.K2_SetActorRotation` (struct :`Yaw` -90.0))))
    (`SceneComponent.K2_SetWorldLocation` (`self.SpringArm`) (`KismetMathLibrary.MakeVector` 0.0 _returnvalue_y _returnvalue_z) false false)))

(event `EnhancedInput|/Game/Input/Actions/IA_Dash`
  (params (ActionValue :type Boolean) (ElapsedSeconds :type "Float (double-precision)") (TriggeredSeconds :type "Float (double-precision)") (InputAction :type "InputAction Object Reference" :default "/Game/Input/Actions/IA_Dash.IA_Dash"))
  (bind _charactermovement (`self.CharacterMovement`))
  ;[0 0 0] IMC Main
  (:`Triggered`
    (if (== 1.0 (`self.Dash Timer var`))
      (`KismetSystemLibrary.PrintString` (`KismetSystemLibrary.GetDisplayName` null))
      (`PaperZDAnimInstance.JumpToNode` (`self.PaperZD ABP`) "Dash" "None")
      (`|ExecutionSequence`
        (:`then_0`
          (set `CharacterMovementComponent.MaxWalkSpeed` 4200.0 _charactermovement)
          (`KismetSystemLibrary.Delay` 0.25)
          (set `CharacterMovementComponent.MaxWalkSpeed` 1000.0 _charactermovement))
        (:`then_1`
          (bind (_direction _dash_timer) (`Timeline|Dash Timer` :!via `PlayFromStart`)
            (:`Update`
              (set `self.Dash Timer var` _dash_timer)))))
      (else
        (`KismetSystemLibrary.PrintText` "Dash Cooldown")))))

(event `EnhancedInput|/Game/Input/Actions/IA_Attack`
  (params (ActionValue :type Boolean) (ElapsedSeconds :type "Float (double-precision)") (TriggeredSeconds :type "Float (double-precision)") (InputAction :type "InputAction Object Reference" :default "/Game/Input/Actions/IA_Attack.IA_Attack"))
  ;[0 0 0] IMC Main
  (:`Triggered`
    (`KismetSystemLibrary.PrintString` (`KismetSystemLibrary.GetDisplayName` InputAction))
    (`PaperZDAnimInstance.JumpToNode` (`self.PaperZD ABP`) "Attack" "None")))

(event `EnhancedInput|/Game/Input/Actions/IA_Parry`
  (params (ActionValue :type Boolean) (ElapsedSeconds :type "Float (double-precision)") (TriggeredSeconds :type "Float (double-precision)") (InputAction :type "InputAction Object Reference" :default "/Game/Input/Actions/IA_Parry.IA_Parry"))
  ;[0 0 0] IMC Main
  (:`Started`
    (`KismetSystemLibrary.PrintString` (`KismetSystemLibrary.GetDisplayName` InputAction))))

(event `EnhancedInput|/Game/Input/Actions/IA_FlyThrough`
  (params (ActionValue :type Boolean) (ElapsedSeconds :type "Float (double-precision)") (TriggeredSeconds :type "Float (double-precision)") (InputAction :type "InputAction Object Reference" :default "/Game/Input/Actions/IA_FlyThrough.IA_FlyThrough"))
  ;[0 0 0] IMC Main
  (:`Triggered`
    (`KismetSystemLibrary.PrintString` (`KismetSystemLibrary.GetDisplayName` InputAction))))

(fn `UserConstructionScript`)