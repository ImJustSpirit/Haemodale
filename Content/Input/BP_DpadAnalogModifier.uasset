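; Input modifier that turns the DualSense D-pad into a WASD-style analog movement stick.
; It rescales the raw X value to a rounded step from 0 to 8, then switches steps 1–8 to 2D axis directions, with unnormalized diagonals.
; Step 0 has no explicit output.
; It is meant only for analog-style use; direction-specific actions belong to the D-pad trigger.
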(fn `ModifyRaw`
  (params (PlayerInput :type "EnhancedPlayerInput Object Reference") (CurrentValue :type "InputActionValue Structure") (DeltaTime :type "Float (single-precision)"))
  (returns (ReturnValue :type "InputActionValue Structure"))
  ;[1 1 1] maps dualsense dpad to function like WASD for movement, do not use if you aren't intending to use the dpad as an analog stick. Use the Dpad TRIGGER if you need for something to only fire if a specific direction is pressed.
  (switch `int` (`KismetMathLibrary.Round` (`KismetMathLibrary.MapRangeClamped` CurrentValue_X 0.0 1.142857 0.0 8.0))
    (:`1`
      (return (make `InputActionValue` 1.0 -1.0 0.0 "Axis2D")))
    (:`2`
      (return (make `InputActionValue` 0.0 -1.0 0.0 "Axis2D")))
    (:`3`
      (return (make `InputActionValue` -1.0 -1.0 0.0 "Axis2D")))
    (:`4`
      (return (make `InputActionValue` -1.0 0.0 0.0 "Axis2D")))
    (:`5`
      (return (make `InputActionValue` -1.0 1.0 0.0 "Axis2D")))
    (:`6`
      (return (make `InputActionValue` 0.0 1.0 0.0 "Axis2D")))
    (:`7`
      (return (make `InputActionValue` 1.0 1.0 0.0 "Axis2D")))
    (:`8`
      (return (make `InputActionValue` 1.0 0.0 0.0 "Axis2D")))))